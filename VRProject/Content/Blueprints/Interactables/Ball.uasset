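; Ball is an interactable physics object that the player can pick up, drop and store in an inventory.
; Pickup disables physics, attaches it to the supplied Hand and shows a widget, while Drop reverses this.
; While held, AddtoInventory replaces the first 0 in the FPS_Controller character's Items array with 1 and destroys the ball, or prints that the inventory is full.
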(event `/Game/Blueprints/Interactables/InteractableInterface.Pickup`
  (params (Hand :type "SceneComponent Object Reference"))
  (`PrimitiveComponent.SetSimulatePhysics` (`self.StaticMesh`) false)
  (`SceneComponent.K2_AttachToComponent` (`self.K2_GetRootComponent`) Hand "None" "KeepWorld" "KeepWorld" "KeepWorld" false)
  (`|ExecutionSequence`
    (:`then_0`
      (bind _output_get (set `self.ObjectGrabbed` true))
      (`KismetSystemLibrary.PrintString` (`KismetStringLibrary.Conv_BoolToString` _output_get)))
    (:`then_1`
      (`SceneComponent.SetVisibility` (`self.Widget`) true false))))

(event `/Game/Blueprints/Interactables/InteractableInterface.Drop`
  (`PrimitiveComponent.SetSimulatePhysics` (`self.StaticMesh`) true)
  (`self.K2_DetachFromActor` "KeepWorld" "KeepWorld" "KeepWorld")
  (`|ExecutionSequence`
    (:`then_0`
      (bind _output_get (set `self.ObjectGrabbed` false))
      (`KismetSystemLibrary.PrintString` (`KismetStringLibrary.Conv_BoolToString` _output_get)))
    (:`then_1`
      (`SceneComponent.SetVisibility` (`self.Widget`) false false))))

(event `/Game/Blueprints/Interactables/InteractableInterface.AddToInventory`
  (if (`self.ObjectGrabbed`)
    (bind _asfps_controller (cast `/Game/Blueprints/FPS_Controller` (`GameplayStatics.GetPlayerCharacter` 0)))
    (bind _items (`/Game/Blueprints/FPS_Controller.Items` _asfps_controller))
    (bind _returnvalue (`KismetArrayLibrary.Array_Find` _items))
    (if (>= _returnvalue 0)
      (`KismetArrayLibrary.Array_Set` _items _returnvalue 1)
      (`self.K2_DestroyActor`)
      (else
        (`KismetSystemLibrary.PrintString` "Inventory is full")))))

(fn `UserConstructionScript`)