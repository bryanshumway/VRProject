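; Key interactable that can be picked up, dropped, or stowed in the player's five-slot inventory.
; Pickup disables mesh physics and attaches the actor to the supplied hand component, while Drop detaches it and restores physics, both updating and printing a grabbed flag.
; AddtoInventory only acts while grabbed, writing the key's item ID into the first empty FPS_Controller slot and destroying the actor, or printing that inventory is full.
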(event `/Game/Blueprints/Interactables/InteractableInterface.Pickup`
  (params (Hand :type "SceneComponent Object Reference"))
  (`PrimitiveComponent.SetSimulatePhysics` (`self.StaticMesh`) false)
  (`SceneComponent.K2_AttachToComponent` (`self.K2_GetRootComponent`) Hand "None" "KeepWorld" "KeepWorld" "KeepWorld" false)
  (bind _output_get (set `self.ObjectGrabbed` true))
  (`KismetSystemLibrary.PrintString` (`KismetStringLibrary.Conv_BoolToString` _output_get)))

(event `/Game/Blueprints/Interactables/InteractableInterface.Drop`
  (`PrimitiveComponent.SetSimulatePhysics` (`self.StaticMesh`) true)
  (`self.K2_DetachFromActor` "KeepWorld" "KeepWorld" "KeepWorld")
  (bind _output_get (set `self.ObjectGrabbed` false))
  (`KismetSystemLibrary.PrintString` (`KismetStringLibrary.Conv_BoolToString` _output_get)))

(event `/Game/Blueprints/Interactables/InteractableInterface.AddToInventory`
  (if (`self.ObjectGrabbed`)
    (bind _asfps_controller (cast `/Game/Blueprints/FPS_Controller` (`GameplayStatics.GetPlayerCharacter` 0)))
    (if (== (`/Game/Blueprints/FPS_Controller.Slot01Item` _asfps_controller) 0)
      (set `/Game/Blueprints/FPS_Controller.Slot01Item` 2 _asfps_controller)
      (`self.K2_DestroyActor` :!label _label)
      (elif (== (`/Game/Blueprints/FPS_Controller.Slot02Item` _asfps_controller) 0)
        (set `/Game/Blueprints/FPS_Controller.Slot02Item` 2 _asfps_controller)
        (goto _label)
        (elif (== (`/Game/Blueprints/FPS_Controller.Slot03Item` _asfps_controller) 0)
          (set `/Game/Blueprints/FPS_Controller.Slot03Item` 2 _asfps_controller)
          (goto _label)
          (elif (== (`/Game/Blueprints/FPS_Controller.Slot04Item` _asfps_controller) 0)
            (set `/Game/Blueprints/FPS_Controller.Slot04Item` 2 _asfps_controller)
            (goto _label)
            (elif (== (`/Game/Blueprints/FPS_Controller.Slot05Item` _asfps_controller) 0)
              (set `/Game/Blueprints/FPS_Controller.Slot05Item` 2 _asfps_controller)
              (goto _label)
              (else
                (`KismetSystemLibrary.PrintString` "Inventory is full")))))))))

(fn `UserConstructionScript`)