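; One-shot welcome trigger that plays Oliver's greeting at the mansion and hands the player the room-finding objectives.
; Any overlap destroys Box1 and hides the EnterMansion_Actor prompt, but only an FPS_Controller starts the voice cue at the FbxScene_Father actor.
; Timed delays step OliverText through two subtitle lines on that actor's widgets.
; It then briefly shows the Objective_01 widget and fills the player's objective texts with rooms to find.
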(event `self.ReceiveActorBeginOverlap`
  (params (OtherActor :type "Actor Object Reference"))
  (`|ExecutionSequence`
    (:`then_0`
      (`ActorComponent.K2_DestroyComponent` (`self.Box1`))
      (cast `/Game/Blueprints/FPS_Controller` OtherActor)
      (bind _outactors (`GameplayStatics.GetAllActorsOfClass` "/Game/Models/NPCs/Father/Father/FbxScene_Father.FbxScene_Father_C"))
      (`GameplayStatics.PlaySoundAtLocation` "/Game/Audio/oliver_welcome_cue.oliver_welcome_cue" (`self.K2_GetActorLocation` (`|GetArrayItem` _outactors)) (struct) 1.0 1.0 0.0 null null null)
      (`|ExecutionSequence`
        (:`then_0`
          (set `self.Oliver_Text` "Well, haven’t seen you in a few years. Come on in.  \nI guess you saw my post in the paper and couldn’t help but be curious with that good ol' realtor's intuition, huh old friend? ")
          (`KismetSystemLibrary.Delay` 9.0)
          (set `self.Oliver_Text` "Feel free to take a look around the place then. \nThe sooner I sell this place the better. Oh, and feel free to ask me any questions, \n I’ll be around if you need me.")
          (`KismetSystemLibrary.Delay` 8.5)
          (set `self.Oliver_Text` "")
          (bind _subtitles (`/Game/Models/NPCs/Father/Father/FbxScene_Father.Subtitles` (`|GetArrayItem` (stale _outactors_3))))
          (`SceneComponent.SetVisibility` _subtitles false false)
          (`SceneComponent.SetVisibility` (`/Game/Models/NPCs/Father/Father/FbxScene_Father.Name` (`|GetArrayItem` (stale _outactors_3))) false false)
          (`|ExecutionSequence`
            (:`then_0`
              (bind _outactors_2 (`GameplayStatics.GetAllActorsOfClass` "/Game/Blueprints/Actors/Objective_01.Objective_01_C"))
              (for _array_element _outactors_2
                (`SceneComponent.SetVisibility` (`/Game/Blueprints/Actors/Objective_01.Widget` _array_element) true false)
                (`KismetSystemLibrary.Delay` 3.0)
                (for _array_element_2 _outactors_2
                  (`SceneComponent.SetVisibility` (`/Game/Blueprints/Actors/Objective_01.Widget` _array_element_2) false false))))
            (:`then_1`
              (bind _asfps_controller (cast `/Game/Blueprints/FPS_Controller` (`GameplayStatics.GetPlayerCharacter` 0)))
              (`|ExecutionSequence`
                (:`then_0`
                  (set `/Game/Blueprints/FPS_Controller.Objective01_Text` "Find the Dining Room" _asfps_controller)
                  (set `/Game/Blueprints/FPS_Controller.Objective06_Text` "Find the Living Room" _asfps_controller)
                  (set `/Game/Blueprints/FPS_Controller.Objective11_Text` "Find the Playroom" _asfps_controller))
                (:`then_1`
                  (set `/Game/Blueprints/FPS_Controller.Objective02_Text` "Find the Kitchen" _asfps_controller)
                  (set `/Game/Blueprints/FPS_Controller.Objective07_Text` "Find the Cellar" _asfps_controller)
                  (set `/Game/Blueprints/FPS_Controller.Objective12_Text` "Find the Attic" _asfps_controller))
                (:`then_2`
                  (set `/Game/Blueprints/FPS_Controller.Objective03_Text` "Find the Ballroom" _asfps_controller)
                  (set `/Game/Blueprints/FPS_Controller.Objective08_Text` "Find the Master Bedroom" _asfps_controller)
                  (set `/Game/Blueprints/FPS_Controller.Objective13_Text` "Find the Kid's Bedroom" _asfps_controller))
                (:`then_3`
                  (set `/Game/Blueprints/FPS_Controller.Objective04_Text` "Find the Study" _asfps_controller)
                  (set `/Game/Blueprints/FPS_Controller.Objective09_Text` "Find the Master Bathroom" _asfps_controller)
                  (set `/Game/Blueprints/FPS_Controller.Objective14_Text` "Find the Kid's Bathroom" _asfps_controller))
                (:`then_4`
                  (set `/Game/Blueprints/FPS_Controller.Objective05_Text` "Find the Library" _asfps_controller)
                  (set `/Game/Blueprints/FPS_Controller.Objective10_Text` "Find the Dressing Room" _asfps_controller))))))
        (:`then_1`
          (bind _outactors_3 (`GameplayStatics.GetAllActorsOfClass` "/Game/Models/NPCs/Father/Father/FbxScene_Father.FbxScene_Father_C"))
          (`SceneComponent.SetVisibility` _subtitles true false)
          (`SceneComponent.SetVisibility` (`/Game/Models/NPCs/Father/Father/FbxScene_Father.Name` (`|GetArrayItem` _outactors_3)) true false))))
    (:`then_1`
      (bind _outactors_4 (`GameplayStatics.GetAllActorsOfClass` "/Game/Blueprints/Actors/EnterMansion_Actor.EnterMansion_Actor_C"))
      (`SceneComponent.SetVisibility` (`/Game/Blueprints/Actors/EnterMansion_Actor.Widget` (`|GetArrayItem` _outactors_4)) false false))))

(fn `UserConstructionScript`)