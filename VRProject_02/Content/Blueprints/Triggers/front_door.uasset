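; One-shot VR trigger that lets the player open the front door with a motion controller grip.
; Input is enabled only while an FPS_Controller actor overlaps it.
; Either grip plays the FrontDoorOpen and DoorKnob level sequences and the DoorOpen sound on the first FbxScene_door found in the level, then destroys the trigger.
; Left and right grips duplicate the same logic.
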(event `self.ReceiveActorBeginOverlap`
  (params (OtherActor :type "Actor Object Reference"))
  (cast `/Game/Blueprints/FPS_Controller` OtherActor)
  (`self.EnableInput` (`GameplayStatics.GetPlayerController` 0)))

(event `self.ReceiveActorEndOverlap`
  (params (OtherActor :type "Actor Object Reference"))
  (cast `/Game/Blueprints/FPS_Controller` OtherActor)
  (`self.DisableInput` (`GameplayStatics.GetPlayerController` 0)))

(event `Key|MotionController_Right_Grip1`
  (params (Key :type "Key Structure"))
  (:`Pressed`
    (bind _outactor (`LevelSequencePlayer.CreateLevelSequencePlayer` "/Game/Animations/FrontDoorOpen.FrontDoorOpen"))
    (`MovieSceneSequencePlayer.Play` (`LevelSequenceActor.SequencePlayer` _outactor))
    (bind _outactors (`GameplayStatics.GetAllActorsOfClass` "/Game/Models/door/FbxScene_door.FbxScene_door_C"))
    (bind _asfbx_scene_door (cast `/Game/Models/door/FbxScene_door` (`|GetArrayItem` _outactors)))
    (`AudioComponent.Play` (`/Game/Models/door/FbxScene_door.DoorOpen` _asfbx_scene_door) 0.0)
    (bind _outactor_2 (`LevelSequencePlayer.CreateLevelSequencePlayer` "/Game/Animations/DoorKnob.DoorKnob"))
    (`MovieSceneSequencePlayer.Play` (`LevelSequenceActor.SequencePlayer` _outactor_2))
    (`self.K2_DestroyActor`)))

(event `Key|MotionController_Left_Grip1`
  (params (Key :type "Key Structure"))
  (:`Pressed`
    (bind _outactor (`LevelSequencePlayer.CreateLevelSequencePlayer` "/Game/Animations/FrontDoorOpen.FrontDoorOpen"))
    (`MovieSceneSequencePlayer.Play` (`LevelSequenceActor.SequencePlayer` _outactor))
    (bind _outactors (`GameplayStatics.GetAllActorsOfClass` "/Game/Models/door/FbxScene_door.FbxScene_door_C"))
    (`AudioComponent.Play` (`/Game/Models/door/FbxScene_door.DoorOpen` (`|GetArrayItem` _outactors)) 0.0)
    (bind _outactor_2 (`LevelSequencePlayer.CreateLevelSequencePlayer` "/Game/Animations/DoorKnob.DoorKnob"))
    (`MovieSceneSequencePlayer.Play` (`LevelSequenceActor.SequencePlayer` _outactor_2))
    (`self.K2_DestroyActor`)))

(fn `UserConstructionScript`)