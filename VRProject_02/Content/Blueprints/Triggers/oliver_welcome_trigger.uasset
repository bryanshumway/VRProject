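; One-shot trigger for Oliver's welcome, which starts the house exploration objective.
; When the player overlaps, it disables its box, hides the entrance widget, plays Oliver's welcome audio and shows timed subtitles.
; Afterwards it activates the first objective with a room checklist, destroys inactive Obj01PM actors and all Obj01Walls, flashes the objective status, and enables asking Oliver questions.
; The player cast feeding Objective01Active runs in a later sequence branch than that write.
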(event `self.ReceiveActorBeginOverlap`
  (params (OtherActor :type "Actor Object Reference"))
  (`|ExecutionSequence`
    (:`then_0`
      (set `PrimitiveComponent.bGenerateOverlapEvents` false (`self.Box1`))
      (bind _asfps_controller (cast `/Game/Blueprints/FPS_Controller` OtherActor))
      (bind _outactors (`GameplayStatics.GetAllActorsOfClass` "/Game/Models/NPCs/Father/Father/FbxScene_Father.FbxScene_Father_C"))
      (`AudioComponent.Play` (`/Game/Models/NPCs/Father/Father/FbxScene_Father.welcome` (`|GetArrayItem` _outactors)) 0.0)
      (`|ExecutionSequence`
        (:`then_0`
          (set `self.Oliver_Text` "Well, haven’t seen you in a few years. Come on in.  \nI guess you saw my post in the paper and couldn’t help but be curious with that good ol' realtor's intuition, huh old friend? ")
          (`KismetSystemLibrary.Delay` 9.0)
          (set `self.Oliver_Text` "Feel free to take a look around the place then. \nThe sooner I sell this place the better. Oh, and feel free to ask me any questions, \n I’ll be around if you need me.")
          (`KismetSystemLibrary.Delay` 8.5)
          (set `self.Oliver_Text` "")
          (`|ExecutionSequence`
            (:`then_0`
              (set `/Game/Blueprints/FPS_Controller.Objective01Active` true (stale _asfps_controller_2))
              (`|ExecutionSequence`
                (:`then_0`
                  (bind _outactors_2 (`GameplayStatics.GetAllActorsOfClass` "/Game/Blueprints/Actors/Walls/PlayerMessages/Obj01PM.Obj01PM_C"))
                  (for _array_element _outactors_2
                    (if (not (`/Game/Blueprints/Actors/Walls/PlayerMessages/Obj01PM.active` _array_element))
                      (`self.K2_DestroyActor` _array_element))))
                (:`then_1`
                  (bind _outactors_3 (`GameplayStatics.GetAllActorsOfClass` "/Game/Blueprints/Actors/Walls/Obj01Walls.Obj01Walls_C"))
                  (for _array_element_2 _outactors_3
                    (`self.K2_DestroyActor` _array_element_2)))))
            (:`then_1`
              (bind _asfps_controller_2 (cast `/Game/Blueprints/FPS_Controller` (`GameplayStatics.GetPlayerCharacter` 0)))
              (`|ExecutionSequence`
                (:`then_0`
                  (set `/Game/Blueprints/FPS_Controller.Objective_1_01_Text` "Check Dining Room" _asfps_controller_2)
                  (set `/Game/Blueprints/FPS_Controller.Objective_1_06_Text` "Check Cellar" _asfps_controller_2))
                (:`then_1`
                  (set `/Game/Blueprints/FPS_Controller.Objective_1_02_Text` "Check Kitchen" _asfps_controller_2)
                  (set `/Game/Blueprints/FPS_Controller.Objective_1_07_Text` "Check Master Bedroom" _asfps_controller_2))
                (:`then_2`
                  (set `/Game/Blueprints/FPS_Controller.Objective_1_03_Text` "Check Living Room" _asfps_controller_2)
                  (set `/Game/Blueprints/FPS_Controller.Objective_1_08_Text` "Check Dressing Room" _asfps_controller_2))
                (:`then_3`
                  (set `/Game/Blueprints/FPS_Controller.Objective_1_04_Text` "Check Library" _asfps_controller_2)
                  (set `/Game/Blueprints/FPS_Controller.Objective_1_09_Text` "Check Kid's Bedroom" _asfps_controller_2))
                (:`then_4`
                  (set `/Game/Blueprints/FPS_Controller.Objective_1_05_Text` "Check Study" _asfps_controller_2)
                  (set `/Game/Blueprints/FPS_Controller.Objective_1_10_Text` "Check Playroom" _asfps_controller_2)
                  (set `/Game/Blueprints/FPS_Controller.Objective_1_11_Text` "Check Attic" _asfps_controller_2))
                (:`then_5`
                  (set `/Game/Blueprints/FPS_Controller.notes_house_01` true _asfps_controller_2))))
            (:`then_2`
              (bind _objectivestatus (`/Game/Blueprints/FPS_Controller.ObjectiveStatus` _asfps_controller))
              (`SceneComponent.SetVisibility` _objectivestatus true false)
              (set `/Game/Blueprints/FPS_Controller.ObjectiveUpdated` "Explore every room" _asfps_controller)
              (`KismetSystemLibrary.Delay` 5.0)
              (`SceneComponent.SetVisibility` _objectivestatus false false))
            (:`then_3`
              (set `self.done` true))
            (:`then_4`
              (`|CreateWidget` "/Game/Blueprints/WidgetSubtitles/oliver_text_01.oliver_text_01_C")
              (set `/Game/Blueprints/FPS_Controller.choice1active` true _asfps_controller_2)
              (set `/Game/Blueprints/FPS_Controller.choice1text` "[Ask question]" _asfps_controller_2))
            (:`then_5`
              (bind _output (`|GetArrayItem` (stale _outactors_4)))
              (set `PrimitiveComponent.bGenerateOverlapEvents` true (`/Game/Models/NPCs/Father/Father/FbxScene_Father.talktrigger` _output)))))
        (:`then_1`
          (bind _outactors_4 (`GameplayStatics.GetAllActorsOfClass` "/Game/Models/NPCs/Father/Father/FbxScene_Father.FbxScene_Father_C"))
          (`SceneComponent.SetVisibility` (`/Game/Models/NPCs/Father/Father/FbxScene_Father.Subtitles` _output) true false)
          (`SceneComponent.SetVisibility` (`/Game/Models/NPCs/Father/Father/FbxScene_Father.Name` _output) true false))))
    (:`then_1`
      (bind _outactors_5 (`GameplayStatics.GetAllActorsOfClass` "/Game/Blueprints/Actors/EnterMansion_Actor.EnterMansion_Actor_C"))
      (`SceneComponent.SetVisibility` (`/Game/Blueprints/Actors/EnterMansion_Actor.Widget` (`|GetArrayItem` _outactors_5)) false false))))

(fn `UserConstructionScript`)