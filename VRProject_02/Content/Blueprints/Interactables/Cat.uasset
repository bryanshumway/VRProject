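; Cat pickup interactable that shows the player a message on overlap and becomes grabbable only if they have already picked up Map 2.
; Pickup turns off physics and collision on the mesh and attaches it to the supplied hand.
; Once grabbed, AddtoInventory writes the cat's item ID into the first empty slot of the FPS_Controller's Items array and destroys the actor, or prints that the inventory is full.
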(event `/Game/Blueprints/Interactables/InteractableInterface.Pickup`
  (params (Hand :type "SceneComponent Object Reference"))
  (if (`self.CanPickup`)
    (`PrimitiveComponent.SetSimulatePhysics` (`self.StaticMesh`) false)
    (`SceneComponent.K2_AttachToComponent` (`self.StaticMesh`) Hand "None" "KeepWorld" "KeepWorld" "KeepWorld" false)
    (set `self.ObjectGrabbed` true)
    (`PrimitiveComponent.SetCollisionEnabled` (`self.StaticMesh`) "NoCollision")))

(event `/Game/Blueprints/Interactables/InteractableInterface.AddToInventory`
  (if (`self.ObjectGrabbed`)
    (bind _asfps_controller (cast `/Game/Blueprints/FPS_Controller` (`GameplayStatics.GetPlayerCharacter` 0)))
    (bind _items (`/Game/Blueprints/FPS_Controller.Items` _asfps_controller))
    (bind _returnvalue (`KismetArrayLibrary.Array_Find` _items))
    (if (>= _returnvalue 0)
      (`KismetArrayLibrary.Array_Set` _items _returnvalue 8)
      (`self.K2_DestroyActor`)
      (else
        (`KismetSystemLibrary.PrintString` "Inventory is full")))))

(event `self.ReceiveActorBeginOverlap`
  (params (OtherActor :type "Actor Object Reference"))
  (bind _asfps_controller (cast `/Game/Blueprints/FPS_Controller` OtherActor))
  (if (`/Game/Blueprints/FPS_Controller.map2pickedup` _asfps_controller)
    (set `/Game/Blueprints/FPS_Controller.PlayerMessage` "There seems to be something here..." _asfps_controller)
    (set `self.CanPickup` true)
    (`KismetSystemLibrary.Delay` 3.0)
    (set `/Game/Blueprints/FPS_Controller.PlayerMessage` "" _asfps_controller)
    (else
      (set `/Game/Blueprints/FPS_Controller.PlayerMessage` "Wow! What a ferocious little cat! This must belong to Rose." _asfps_controller)
      (`KismetSystemLibrary.Delay` 5.0)
      (set `/Game/Blueprints/FPS_Controller.PlayerMessage` "" _asfps_controller))))

(fn `UserConstructionScript`)