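; Interactable map pickup that the player can grab by hand and store in an inventory slot.
; Pickup turns off mesh physics and attaches the actor to the grabbing hand.
; AddtoInventory, allowed once grabbed and shortly after BeginPlay, writes the item ID into the first empty of ten FPS_Controller slots.
; The actor is destroyed after filling slots one to seven, but remains for slots eight to ten.
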(event `self.ReceiveBeginPlay`
  (`KismetSystemLibrary.Delay` 0.1)
  (set `self.CanPickup` true))

(event `/Game/Blueprints/Interactables/InteractableInterface.Pickup`
  (params (Hand :type "SceneComponent Object Reference"))
  (`PrimitiveComponent.SetSimulatePhysics` (`self.StaticMesh`) false)
  (`SceneComponent.K2_AttachToComponent` (`self.K2_GetRootComponent`) Hand "None" "KeepWorld" "KeepWorld" "KeepWorld" false)
  (bind _output_get (set `self.ObjectGrabbed` true))
  (`KismetSystemLibrary.PrintString` (`KismetStringLibrary.Conv_BoolToString` _output_get)))

(event `/Game/Blueprints/Interactables/InteractableInterface.AddToInventory`
  (if (`self.ObjectGrabbed`)
    (if (`self.CanPickup`)
      (bind _asfps_controller (cast `/Game/Blueprints/FPS_Controller` (`GameplayStatics.GetPlayerCharacter` 0)))
      (if (== (`/Game/Blueprints/FPS_Controller.Slot01Item` _asfps_controller) 0)
        (set `/Game/Blueprints/FPS_Controller.Slot01Item` 2 _asfps_controller)
        (`self.K2_DestroyActor` :!label _label)
        (elif (== (`/Game/Blueprints/FPS_Controller.Slot02Item` _asfps_controller) 0)
          (set `/Game/Blueprints/FPS_Controller.Slot02Item` 2 _asfps_controller)
          (goto _label)
          (elif (== (`/Game/Blueprints/FPS_Controller.Slot03Item` _asfps_controller) 0)
            (set `/Game/Blueprints/FPS_Controller.Slot03Item` 2 _asfps_controller)
            (goto _label)
            (elif (== (`/Game/Blueprints/FPS_Controller.Slot04Item` _asfps_controller) 0)
              (set `/Game/Blueprints/FPS_Controller.Slot04Item` 2 _asfps_controller)
              (goto _label)
              (elif (== (`/Game/Blueprints/FPS_Controller.Slot05Item` _asfps_controller) 0)
                (set `/Game/Blueprints/FPS_Controller.Slot05Item` 2 _asfps_controller)
                (goto _label)
                (elif (== (`/Game/Blueprints/FPS_Controller.Slot06Item` _asfps_controller) 0)
                  (set `/Game/Blueprints/FPS_Controller.Slot06Item` 2 _asfps_controller)
                  (goto _label)
                  (elif (== (`/Game/Blueprints/FPS_Controller.Slot07Item` _asfps_controller) 0)
                    (set `/Game/Blueprints/FPS_Controller.Slot07Item` 2 _asfps_controller)
                    (goto _label)
                    (elif (== (`/Game/Blueprints/FPS_Controller.Slot08Item` _asfps_controller) 0)
                      (set `/Game/Blueprints/FPS_Controller.Slot08Item` 2 _asfps_controller)
                      (elif (== (`/Game/Blueprints/FPS_Controller.Slot09Item` _asfps_controller) 0)
                        (set `/Game/Blueprints/FPS_Controller.Slot09Item` 2 _asfps_controller)
                        (elif (== (`/Game/Blueprints/FPS_Controller.Slot10Item` _asfps_controller) 0)
                          (set `/Game/Blueprints/FPS_Controller.Slot10Item` 2 _asfps_controller))))))))))))))

(fn `UserConstructionScript`)