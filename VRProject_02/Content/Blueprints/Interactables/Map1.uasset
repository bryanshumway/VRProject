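; Map1 is an interactable item that the player can pick up in hand and store in the FPS_Controller inventory.
; Pickup disables physics and collision on the static mesh, attaches it to the supplied hand and flags it as grabbed.
; AddtoInventory, only while grabbed, writes the map's item ID into the first empty Items slot and destroys the actor, or prints that the inventory is full.
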(event `/Game/Blueprints/Interactables/InteractableInterface.Pickup`
  (params (Hand :type "SceneComponent Object Reference"))
  (`PrimitiveComponent.SetSimulatePhysics` (`self.StaticMesh`) false)
  (`SceneComponent.K2_AttachToComponent` (`self.StaticMesh`) Hand "None" "KeepWorld" "KeepWorld" "KeepWorld" false)
  (set `self.ObjectGrabbed` true)
  (`PrimitiveComponent.SetCollisionEnabled` (`self.StaticMesh`) "NoCollision"))

(event `/Game/Blueprints/Interactables/InteractableInterface.AddToInventory`
  (if (`self.ObjectGrabbed`)
    (bind _asfps_controller (cast `/Game/Blueprints/FPS_Controller` (`GameplayStatics.GetPlayerCharacter` 0)))
    (bind _items (`/Game/Blueprints/FPS_Controller.Items` _asfps_controller))
    (bind _returnvalue (`KismetArrayLibrary.Array_Find` _items))
    (if (>= _returnvalue 0)
      (`KismetArrayLibrary.Array_Set` _items _returnvalue 7)
      (`self.K2_DestroyActor`)
      (else
        (`KismetSystemLibrary.PrintString` "Inventory is full")))))

(fn `UserConstructionScript`)