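; Interactable attic key that the player can grab and store in their inventory.
; Pickup turns off physics and collision on the SkeletonKey component and attaches it to the given hand.
; Once grabbed, AddtoInventory writes the key's item ID into the first empty (zero) slot of the FPS_Controller character's Items array and destroys the actor.
; If no slot is free, it prints that the inventory is full.
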(event `/Game/Blueprints/Interactables/InteractableInterface.Pickup`
  (params (Hand :type "SceneComponent Object Reference"))
  (`PrimitiveComponent.SetSimulatePhysics` (`self.Skeleton_Key`) false)
  (`SceneComponent.K2_AttachToComponent` (`self.Skeleton_Key`) Hand "None" "KeepWorld" "KeepWorld" "KeepWorld" false)
  (set `self.ObjectGrabbed` true)
  (`PrimitiveComponent.SetCollisionEnabled` (`self.Skeleton_Key`) "NoCollision"))

(event `/Game/Blueprints/Interactables/InteractableInterface.AddToInventory`
  (if (`self.ObjectGrabbed`)
    (bind _asfps_controller (cast `/Game/Blueprints/FPS_Controller` (`GameplayStatics.GetPlayerCharacter` 0)))
    (bind _items (`/Game/Blueprints/FPS_Controller.Items` _asfps_controller))
    (bind _returnvalue (`KismetArrayLibrary.Array_Find` _items))
    (if (>= _returnvalue 0)
      (`KismetArrayLibrary.Array_Set` _items _returnvalue 6)
      (`self.K2_DestroyActor`)
      (else
        (`KismetSystemLibrary.PrintString` "Inventory is full")))))

(fn `UserConstructionScript`)