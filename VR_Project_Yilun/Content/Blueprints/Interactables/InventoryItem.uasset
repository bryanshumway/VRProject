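; An inventory pickup actor that the player can collect, identified by an ItemID.
; On BeginPlay it looks up its row in the InventoryData table and sets its static mesh from that row.
; Pickup casts the player character to FPS_Controller, adds the ItemID to its PlayerInventory and destroys the actor.
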(event `self.ReceiveBeginPlay`
  (bind _returnvalue (`|GetDataTableRow` "/Game/Data/InventoryData.InventoryData" (`self.ItemID`))
    (:`then`
      (`StaticMeshComponent.SetStaticMesh` (`self.StaticMesh`) (`.Mesh_19_7CD451A44A887B603794088732690BB1` (break `/Game/Data/InventoryItem` _returnvalue))))))

(event `/Game/Blueprints/Interactables/InteractableInterface.Pickup`
  (params (Hand :type "SceneComponent Object Reference"))
  (bind _asfps_controller (cast `/Game/Blueprints/FPS_Controller` (`GameplayStatics.GetPlayerCharacter` 0)))
  (`KismetArrayLibrary.Array_Add` (`/Game/Blueprints/FPS_Controller.PlayerInventory` _asfps_controller) (`self.ItemID`))
  (`self.K2_DestroyActor`))

(fn `UserConstructionScript`
  (`parent.UserConstructionScript`))