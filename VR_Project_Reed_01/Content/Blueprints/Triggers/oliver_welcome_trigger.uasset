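; One-shot trigger that plays Oliver's welcome dialogue with timed subtitles when the player overlaps it.
; The first overlapping actor destroys the box before the FPS_Controller cast, so any actor can use it up.
; The voice cue plays at the first FbxScene_Father actor's location.
; A Sequence shows that actor's subtitle and name components while Delays step OliverText through two lines, then clear and hide them.
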(event `self.ReceiveActorBeginOverlap`
  (params (OtherActor :type "Actor Object Reference"))
  (`ActorComponent.K2_DestroyComponent` (`self.Box1`))
  (cast `/Game/Blueprints/FPS_Controller` OtherActor)
  (bind _outactors (`GameplayStatics.GetAllActorsOfClass` "/Game/Models/NPCs/Father/Father/FbxScene_Father.FbxScene_Father_C"))
  (`GameplayStatics.PlaySoundAtLocation` "/Game/Audio/oliver_welcome_cue.oliver_welcome_cue" (`self.K2_GetActorLocation` (`|GetArrayItem` _outactors)) (struct) 1.0 1.0 0.0 null null null)
  (`|ExecutionSequence`
    (:`then_0`
      (set `self.Oliver_Text` "Well, haven’t seen you in a few years. Come on in.  \nI guess you saw my post in the paper and couldn’t help but be curious with that good ol' realtor's intuition, huh old friend? ")
      (`KismetSystemLibrary.Delay` 9.0)
      (set `self.Oliver_Text` "Feel free to take a look around the place then. \nThe sooner I sell this place the better. Oh, and feel free to ask me any questions, \n I’ll be around if you need me.")
      (`KismetSystemLibrary.Delay` 8.5)
      (set `self.Oliver_Text` "")
      (bind _subtitles (`/Game/Models/NPCs/Father/Father/FbxScene_Father.Subtitles` (`|GetArrayItem` (stale _outactors_2))))
      (`SceneComponent.SetVisibility` _subtitles false false)
      (`SceneComponent.SetVisibility` (`/Game/Models/NPCs/Father/Father/FbxScene_Father.Name` (`|GetArrayItem` (stale _outactors_2))) false false))
    (:`then_1`
      (bind _outactors_2 (`GameplayStatics.GetAllActorsOfClass` "/Game/Models/NPCs/Father/Father/FbxScene_Father.FbxScene_Father_C"))
      (`SceneComponent.SetVisibility` _subtitles true false)
      (`SceneComponent.SetVisibility` (`/Game/Models/NPCs/Father/Father/FbxScene_Father.Name` (`|GetArrayItem` _outactors_2)) true false))))

(fn `UserConstructionScript`)